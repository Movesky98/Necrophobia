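; BP_BarrelExplosive is a destructible barrel actor that explodes visually and audibly once damage depletes its health.
; AnyDamage subtracts damage from Health and, at zero or below, spawns an attached explosion particle, reveals a hidden decal, destroys the static mesh and requests an explosion sound on that destroyed component.
; It applies no damage to surroundings and has no guard against further hits retriggering the sequence.
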(event EventBeginPlay
  (|CallParentFunction) ; This node is disabled and will not be called.\nDrag off pins to build functionality.
)

(event Collision|EventActorBeginOverlap
  (params (OtherActor :type Actor%20Object%20Reference))
  (|CallParentFunction OtherActor) ; This node is disabled and will not be called.\nDrag off pins to build functionality.
)

(event EventTick
  (params (DeltaSeconds :type Float%20%28single-precision%29))
  (|CallParentFunction DeltaSeconds) ; This node is disabled and will not be called.\nDrag off pins to build functionality.
)

(event Game|Damage|EventAnyDamage
  (params (Damage :type Float%20%28single-precision%29) (DamageType :type Damage%20Type%20Object%20Reference) (InstigatedBy :type Controller%20Object%20Reference) (DamageCauser :type Actor%20Object%20Reference))
  (bind _output_get (Variables|Default|SetHealth (- (Variables|Default|GetHealth) Damage)))
  (if (<= _output_get 0.0)
    (Effects|SpawnEmitterAttached (Variables|Default|GetExplosion_Particle) (Variables|Default|GetStaticMesh) "None")
    (Development|SetHiddeninGame (Variables|Default|GetDecal) false false)
    (Components|DestroyComponent (Variables|Default|GetStaticMesh))
    (Audio|SpawnSoundAttached "/Game/Impacts/BluePrints/FirstPersonBP/FirstPerson/Audio/Explosion_Cue.Explosion_Cue" (Variables|Default|GetStaticMesh))))

(fn ConstructionScript
  (|CallParentFunction))