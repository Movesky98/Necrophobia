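; BP_BulletHole is a short-lived impact actor that spawns an animated bullet hole decal.
; On BeginPlay it spawns a decal from its material and transform variables, with a fixed lifespan, and creates a dynamic material instance.
; A timeline drives that instance's opacity and two base colors.
; The actor destroys itself when the timeline finishes, or immediately if either material is invalid.
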(event EventBeginPlay
  (bind _decalmaterial (Variables|Default|GetDecalMaterial))
  (bind _decaltransform (Variables|Default|GetDecalTransform))
  (Utilities|IsValid _decalmaterial
    (:Is%20Valid
      (bind _returnvalue (Rendering|Decal|SpawnDecalatLocation _decalmaterial (.scale _decaltransform) (.location _decaltransform) (.rotation _decaltransform) 3.0))
      (bind _returnvalue_2 (Rendering|Material|CreateDynamicMaterialInstance _returnvalue :!class /Script/Engine.DecalComponent))
      (Utilities|IsValid _returnvalue_2
        (:Is%20Valid
          (bind (_direction _opacity _base_color _base_color1) (Timeline|Decal PlayFromStart)
            (:Update
              (Rendering|Material|SetScalarParameterValue _returnvalue_2 "Opacity" _opacity :!class /Script/Engine.MaterialInstanceDynamic)
              (Rendering|Material|SetVectorParameterValue _returnvalue_2 "Base_Color" (Math|Conversions|ToLinearColor(Vector) _base_color) :!class /Script/Engine.MaterialInstanceDynamic)
              (Rendering|Material|SetVectorParameterValue _returnvalue_2 "Base_Color1" (Math|Conversions|ToLinearColor(Vector) _base_color1) :!class /Script/Engine.MaterialInstanceDynamic))
            (:Finished
              (Actor|DestroyActor :!label _label))))
        (:Is%20Not%20Valid
          (goto _label))))
    (:Is%20Not%20Valid
      (goto _label))))

(fn ConstructionScript)